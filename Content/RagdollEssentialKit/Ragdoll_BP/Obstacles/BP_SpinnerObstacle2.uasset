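; Spinning obstacle that knocks the ragdoll character into ragdoll on contact.
; A Timeline started at BeginPlay acts as a ticker, adding a fixed pitch step to the Scene component on each update, so speed depends on frame rate.
; Three box triggers each cast the overlapping actor to BP_RagdollCharacter and call ActivateRagdoll on its RagdollComponent.
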(event `self.ReceiveBeginPlay`
  (`Timeline|Timeline`
    (:`Update`
      (bind _output_get (set `self.Rotation` (+ (`self.Rotation`) 1.0)))
      (`SceneComponent.K2_SetRelativeRotation` (`self.Scene`) (`KismetMathLibrary.MakeRotator` 0.0 _output_get) false false))))

(event `self.Box.OnComponentBeginOverlap`
  (params (OverlappedComponent :type "PrimitiveComponent Object Reference") (OtherActor :type "Actor Object Reference") (OtherComp :type "PrimitiveComponent Object Reference") (OtherBodyIndex :type Integer) (bFromSweep :type Boolean) (SweepResult :type "HitResult Structure (by ref)"))
  (bind _asbp_ragdoll_character (cast `/Game/RagdollEssentialKit/Ragdoll_BP/Player/BP_RagdollCharacter` OtherActor))
  (`/Game/RagdollEssentialKit/Ragdoll_BP/AC_RagdollComponent.ActivateRagdoll` (`/Game/RagdollEssentialKit/Ragdoll_BP/Player/BP_RagdollCharacter.RagdollComponent` _asbp_ragdoll_character)))

(event `self.Box2.OnComponentBeginOverlap`
  (params (OverlappedComponent :type "PrimitiveComponent Object Reference") (OtherActor :type "Actor Object Reference") (OtherComp :type "PrimitiveComponent Object Reference") (OtherBodyIndex :type Integer) (bFromSweep :type Boolean) (SweepResult :type "HitResult Structure (by ref)"))
  (bind _asbp_ragdoll_character (cast `/Game/RagdollEssentialKit/Ragdoll_BP/Player/BP_RagdollCharacter` OtherActor))
  (`/Game/RagdollEssentialKit/Ragdoll_BP/AC_RagdollComponent.ActivateRagdoll` (`/Game/RagdollEssentialKit/Ragdoll_BP/Player/BP_RagdollCharacter.RagdollComponent` _asbp_ragdoll_character)))

(event `self.Box1.OnComponentBeginOverlap`
  (params (OverlappedComponent :type "PrimitiveComponent Object Reference") (OtherActor :type "Actor Object Reference") (OtherComp :type "PrimitiveComponent Object Reference") (OtherBodyIndex :type Integer) (bFromSweep :type Boolean) (SweepResult :type "HitResult Structure (by ref)"))
  (bind _asbp_ragdoll_character (cast `/Game/RagdollEssentialKit/Ragdoll_BP/Player/BP_RagdollCharacter` OtherActor))
  (`/Game/RagdollEssentialKit/Ragdoll_BP/AC_RagdollComponent.ActivateRagdoll` (`/Game/RagdollEssentialKit/Ragdoll_BP/Player/BP_RagdollCharacter.RagdollComponent` _asbp_ragdoll_character)))

(fn `UserConstructionScript`)