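; Star is a goal actor that ends the run when a BP_RagdollCharacter overlaps its static mesh.
; On overlap it plays a bonus sound, reads the time from the WBP_PressFKey widget and debug-prints it.
; It passes that time to a new Win widget, which replaces all other widgets on screen.
; The star then destroys itself and the mouse cursor is shown.
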(event `self.StaticMesh.OnComponentBeginOverlap`
  (params (OverlappedComponent :type "PrimitiveComponent Object Reference") (OtherActor :type "Actor Object Reference") (OtherComp :type "PrimitiveComponent Object Reference") (OtherBodyIndex :type Integer) (bFromSweep :type Boolean) (SweepResult :type "HitResult Structure (by ref)"))
  (cast `/Game/Ragdoll/Ragdoll_BP/Player/BP_RagdollCharacter` OtherActor)
  (`GameplayStatics.PlaySoundAtLocation` "/Game/Music/game-bonus-144751.game-bonus-144751" (`self.K2_GetActorLocation`) (struct) 1.0 1.0 0.0 null null null null)
  (cast `/Game/Ragdoll/Ragdoll_BP/Player/BP_RagdollCharacter` OtherActor)
  (bind _foundwidgets (`WidgetBlueprintLibrary.GetAllWidgetsOfClass` "/Game/Ragdoll/UI/WBP_PressFKey.WBP_PressFKey_C"))
  (bind _output (`/Game/Ragdoll/UI/WBP_PressFKey.getTime` _foundwidgets))
  (`KismetSystemLibrary.PrintText` (`KismetTextLibrary.Conv_DoubleToText` _output "HalfToEven"))
  (bind _returnvalue (`|CreateWidget` "/Game/Blueprints/Win.Win_C"))
  (bind _aswin (cast `/Game/Blueprints/Win` _returnvalue))
  (`/Game/Blueprints/Win.SetFinalTime` _aswin _output)
  (`WidgetLayoutLibrary.RemoveAllWidgets`)
  (`UserWidget.AddToViewport` _returnvalue 0)
  (`self.K2_DestroyActor`)
  (set `PlayerController.bShowMouseCursor` true (`GameplayStatics.GetPlayerController` 0)))

(fn `UserConstructionScript`)